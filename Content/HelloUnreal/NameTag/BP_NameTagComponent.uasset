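; BP_NameTagComponent gives its owning Character a name tag widget that follows it and shows its HP.
; On BeginPlay it creates the widget in the viewport, binds to the owner's StatComponent HP dispatcher and pushes initial HP, printing a warning if that component is missing.
; Each Tick passes the component's world location to the viewport widget to update the tag.
; EndPlay removes the widget.
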(event EventBeginPlay
  (bind _returnvalue (Components|GetOwner))
  (bind _returnvalue_2 (Actor|GetComponentbyClass _returnvalue "/Game/HelloUnreal/AI/StatComponent.StatComponent_C"))
  (CallFunction|CreateWidget)
  (Utilities|IsValid _returnvalue_2
    (:Is%20Valid
      (EventDispatchers|BindEventtoEventDispatcherUpdateHp _returnvalue_2 (EventDispatchers|CreateEvent :!event UpdateHp))
      (CallFunction|UpdateHp (Variables|/Game/HelloUnreal/AI/StatComponent.StatComponent_C|GetCurHp _returnvalue_2) (Variables|/Game/HelloUnreal/AI/StatComponent.StatComponent_C|GetMaxHp _returnvalue_2)))
    (:Is%20Not%20Valid
      (Development|PrintString "Owner Has No StatComponent!" true true "(R=1.000000,G=0.000000,B=0.000000,A=1.000000)"))))

(event EventTick
  (params (DeltaSeconds :type Float%20%28single-precision%29))
  (bind _nametagwidget (Variables|Default|GetNameTagWidget)
    (:then
      (Default|UpdateNameTag _nametagwidget (Transformation|GetWorldLocation)))
    (:else)))

(event EventEndPlay
  (params (EndPlayReason :type EEndPlayReason%20Enum :default "Destroyed"))
  (bind _nametagwidget (Variables|Default|GetNameTagWidget)
    (:then
      (Widget|RemovefromParent _nametagwidget))
    (:else)))

(fn UpdateHp
  (params (CurHp :type Float%20%28double-precision%29) (MaxHp :type Float%20%28double-precision%29))
  (Default|UpdateHp (Variables|Default|GetNameTagWidget) CurHp MaxHp))

(fn CreateWidget
  (bind _ascharacter (Utilities|Casting|CastToCharacter (Components|GetOwner)))
  (bind _returnvalue (UserInterface|CreateWidget "/Game/HelloUnreal/NameTag/NameTagWidget.NameTagWidget_C" 0 _ascharacter))
  (bind _output_get (Variables|Default|SetNameTagWidget _returnvalue))
  (UserInterface|Viewport|AddtoViewport _output_get 0))