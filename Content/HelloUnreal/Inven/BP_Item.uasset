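; BP_Item is an inventory item actor identified by a row name in DT_Item.
; Its construction script looks up that row and applies the row's static mesh.
; GetItem passes the row name to AddItem on the character's InvenComponent, then destroys the actor when that call returns false.
; A similar pickup chain in the event graph is unconnected and never runs.
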(fn ConstructionScript
  (bind _returnvalue (Utilities|GetDataTableRow "/Game/HelloUnreal/Inven/DT_Item.DT_Item" (Variables|Default|GetItemRowName))
    (:then
      (Components|StaticMesh|SetStaticMesh (Variables|Default|GetStaticMesh) (.StaticMesh (Utilities|Struct|BreakST_Item _returnvalue))))))

(fn GetItem
  (params (Character :type Character%20Object%20Reference))
  (bind _returnvalue (Actor|GetComponentbyClass Character "/Game/HelloUnreal/Inven/InvenComponent.InvenComponent_C"))
  (Utilities|IsValid _returnvalue
    (:Is%20Valid
      (bind _bisfail (Default|AddItem _returnvalue (Variables|Default|GetItemRowName)))
      (if (not _bisfail)
        (Actor|DestroyActor)))))