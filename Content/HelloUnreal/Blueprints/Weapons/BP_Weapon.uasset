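; Weapon actor that a character can carry and strike with, configured from DT_Weapon rows.
; The construction script applies the named row's mesh for placement preview, while BeginPlay picks a random row if none is set.
; Attach functions snap it to character mesh sockets, and detaching drops it with physics.
; EventNotifyHit sphere-traces at the "hit" socket and applies fixed damage, crediting the holder's controller.
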(event EventBeginPlay
  (if (== (Variables|Default|GetWeaponRowName) "None")
    (bind _outrownames (DataTable|GetDataTableRowNames "/Game/HelloUnreal/Data/DT_Weapon.DT_Weapon"))
    (bind _returnvalue (Utilities|GetDataTableRow "/Game/HelloUnreal/Data/DT_Weapon.DT_Weapon" (.OutItem (Utilities|Array|Random _outrownames)))
      (:then
        (bind _output_get (Variables|Default|SetWeaponData _returnvalue))
        (Components|StaticMesh|SetStaticMesh (Variables|Default|GetWeapon) (.StaticMesh (Utilities|Struct|BreakST_Weapon _output_get)))))))

(fn ConstructionScript
  ;[0.15 0.15 0.15 0.5] 생성스크립트에 있어야 배치 시 Mesh가 즉시 반영됨
  (bind _returnvalue (Utilities|GetDataTableRow "/Game/HelloUnreal/Data/DT_Weapon.DT_Weapon" (Variables|Default|GetWeaponRowName))
    (:then
      (bind _output_get (Variables|Default|SetWeaponData _returnvalue))
      (Components|StaticMesh|SetStaticMesh (Variables|Default|GetWeapon) (.StaticMesh (Utilities|Struct|BreakST_Weapon _output_get))))))

(fn EventReleaseF
  (return false))

(fn EventPressF
  (params (Character :type Character%20Object%20Reference))
  (Transformation|AttachComponentToComponent (Variables|/Script/Engine.Character|GetMesh Character) "weapon" "SnapToTarget" "SnapToTarget" "KeepWorld" true)
  (return false))

(fn AttachtoChar
  (params (Character :type Character%20Object%20Reference))
  ;[0.15 0.15 0.15 0.5] 변수
  (Variables|Default|SetCharacter Character)
  (Transformation|AttachComponentToComponent (Variables|/Script/Engine.Character|GetMesh Character) (.socket (Variables|Default|GetWeaponData)) "SnapToTarget" "SnapToTarget" "KeepWorld" true)
  (return false))

(fn DetachtoChar
  (params (Character :type Character%20Object%20Reference))
  (Transformation|DetachFromActor "KeepWorld" "KeepWorld" "KeepWorld")
  (Physics|SetSimulatePhysics (Variables|Default|GetWeapon) true)
  (Variables|Default|SetCharacter 0)
  (return false))

(fn EventNotifyHit
  (bind _weapon (Variables|Default|GetWeapon))
  (bind _returnvalue (Transformation|GetSocketLocation _weapon "hit"))
  (bind _outhit (Collision|SphereTraceForObjects _returnvalue _returnvalue 5e+01 (Utilities|Array|MakeArray "ObjectTypeQuery2") false 0 "ForDuration"))
  (Game|Damage|ApplyDamage (.HitActor (Collision|BreakHitResult _outhit)) 1e+01 (Pawn|GetController (Variables|Default|GetCharacter)) self)
  (return false))