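; BP_Switch is a switch that turns play and stop on or off for a list of actors.
; Its ToggleSwitch event flips the Toggle boolean, then loops over the Actors array and passes the new state to EventPlay on elements that cast to the BPI_PlayStop interface.
; Nothing in this graph triggers the event, and the overlap logging and array example nodes are disconnected leftovers.
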(event Custom|ToggleSwitch
  (Variables|Default|SetbToggle (not (Variables|Default|GetbToggle)))
  (for _array_element (Variables|Default|GetActors)
    (bind _asbpi_play_stop (Utilities|Casting|CastToBPI_PlayStop _array_element))
    (Default|EventPlay _asbpi_play_stop (Variables|Default|GetbToggle))))

(fn ConstructionScript)