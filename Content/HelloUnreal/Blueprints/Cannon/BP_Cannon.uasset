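; BP_Cannon is a cannon actor that toggles automatic firing each time something begins overlapping its StaticMesh.
; Toggling on fires immediately and starts a looping one-second timer on ShootCannon by function name; toggling off clears that timer.
; ShootCannon spawns a BP_CannonBall at the Arrow component's world location and rotation.
; Unconnected pause and unpause timer nodes remain in the event graph.
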(event OnComponentBeginOverlap(StaticMesh)
  (params (OverlappedComponent :type Primitive%20Component%20Object%20Reference) (OtherActor :type Actor%20Object%20Reference) (OtherComp :type Primitive%20Component%20Object%20Reference) (OtherBodyIndex :type Integer) (bFromSweep :type Boolean) (SweepResult :type Hit%20Result%20Structure%20%28by%20ref%29))
  ;[0.15 0.15 0.15 0.5] Toggle
  (bind _output_get (Variables|Default|SetbToggle (not (Variables|Default|GetbToggle))))
  (if _output_get
    ;[0.15 0.15 0.15 0.5] FirstShoot
    (CallFunction|ShootCannon)
    (Utilities|Time|SetTimerbyFunctionName 0 "ShootCannon" 1.0 true)
    (else
      (Utilities|Time|ClearTimerbyFunctionName 0 "ShootCannon"))))

(fn ConstructionScript)

(fn ShootCannon
  (bind _arrow (Variables|Default|GetArrow))
  (bind _returnvalue (Transformation|GetWorldTransform _arrow))
  (Game|SpawnActorfromClass "/Game/HelloUnreal/Blueprints/Cannon/BP_CannonBall.BP_CannonBall_C" (Math|Transform|MakeTransform (.location _returnvalue) (.rotation _returnvalue) "1.000000,1.000000,1.000000") "Undefined" "MultiplyWithRoot" 0 0))