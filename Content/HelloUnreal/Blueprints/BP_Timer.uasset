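; BP_Timer is a count-up timer that displays elapsed time as MM:SS on a TextRender component.
; While IsPlay is true, Tick adds delta time scaled by Speed to TotalDeltaSeconds, then refreshes the text.
; The FloatToStr00 helper zero-pads minutes and seconds by building each from floored tens and ones digits.
; An earlier inline digit-formatting chain and some rounding nodes remain unused in the graph.
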(event EventTick
  (params (DeltaSeconds :type Float%20%28single-precision%29))
  (if (Variables|Default|GetbIsPlay)
    (bind _output_get (Variables|Default|SetTotalDeltaSeconds (+ (* DeltaSeconds (Variables|Default|GetSpeed)) (Variables|Default|GetTotalDeltaSeconds))))
    (Rendering|Components|TextRender|SetText (Variables|Default|GetTextRender) (Utilities|Text|ToText(String) (Utilities|String|Append (CallFunction|FloattoStr00 (/ _output_get 6e+01)) ":" (CallFunction|FloattoStr00 (Math|Float|%(Float) _output_get 6e+01)))))))

(fn ConstructionScript)

(fn FloattoStr00
  (params (Number :type Float%20%28double-precision%29))
  (return (Utilities|String|Append (Utilities|String|ToString(Integer) (Math|Float|Floor (/ Number 1e+01))) (Utilities|String|ToString(Integer) (Math|Float|Floor (Math|Float|%(Float) Number 1e+01))))))