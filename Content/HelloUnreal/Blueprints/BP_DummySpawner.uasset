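; Spawner actor that keeps a BP_Dummy in the level, spawning one at its own location and rotation on BeginPlay.
; SpawnDummy binds to each dummy's built-in OnDestroyed dispatcher, so destruction leads to a respawn through a short SetTimerByFunctionName delay.
; An alternative binding to a custom death dispatcher is left disconnected, alongside an EventDeath handler that duplicates the respawn timer.
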(event EventBeginPlay
  (CallFunction|SpawnDummy))

(fn ConstructionScript)

(fn EventDeath
  (Utilities|Time|SetTimerbyFunctionName 0 "SpawnDummy" 3.0))

(fn SpawnDummy
  (bind _returnvalue (Transformation|GetActorTransform))
  (bind _returnvalue_2 (Game|SpawnActorfromClass "/Game/HelloUnreal/Blueprints/BP_Dummy.BP_Dummy_C" (Math|Transform|MakeTransform (.location _returnvalue) (.rotation _returnvalue) "1.000000,1.000000,1.000000") "Undefined" "MultiplyWithRoot" 0 0))
  ;[0.15 0.15 0.15 0.5] Actor 내장 Dispatcher
  (Game|BindEventtoOnDestroyed _returnvalue_2 (EventDispatchers|CreateEvent :!event EventDestroy)))

(fn EventDestroy
  (params (DestroyedActor :type Actor%20Object%20Reference))
  (Utilities|Time|SetTimerbyFunctionName 0 "SpawnDummy" 3.0))