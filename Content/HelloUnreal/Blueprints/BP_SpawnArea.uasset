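; BP_SpawnArea is an actor that scatters spawned actors at random points inside its Box component.
; Its SpawnToArea event runs two loops in sequence: one spawns five BP_Rock actors, the other attempts ten spawns with no class set.
; Each location comes from RandomPointInBoundingBox using the box's world location and scaled extent.
; Unconnected leftover nodes hold a counter-capped rock spawn with a "Too Many Stones!" message and an empty loop.
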(event Custom|SpawnToArea
  (bind _box (Variables|Default|GetBox))
  (bind _returnvalue (Transformation|GetWorldLocation _box))
  (bind _returnvalue_2 (Components|Box|GetScaledBoxExtent _box))
  (bind _returnvalue_3 (Math|Random|RandomPointinBoundingBox _returnvalue _returnvalue_2))
  (Utilities|FlowControl|Sequence
    (:then_0
      (for _index (range 1 5)
        (Game|SpawnActorfromClass "/Game/HelloUnreal/Blueprints/BP_Rock.BP_Rock_C" (Math|Transform|MakeTransform _returnvalue_3 "0, 0, 0" "1.000000,1.000000,1.000000") "Undefined" "MultiplyWithRoot" 0 0)))
    (:then_1
      (for _index_2 (range 1 10)
        (Game|SpawnActorfromClass "/Game/HelloUnreal/Blueprints/BP_RedBall.BP_RedBall_C" (Math|Transform|MakeTransform _returnvalue_3 "0, 0, 0" "1.000000,1.000000,1.000000") "Undefined" "MultiplyWithRoot" 0 0)))))

(fn ConstructionScript)