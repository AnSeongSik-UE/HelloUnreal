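; BP_Dummy is a damageable target actor that displays its remaining health as it takes damage.
; On AnyDamage it subtracts damage from CurrentHp and writes the value to a text render component.
; It casts its widget component's widget to DummyWidget and sets that widget's CurrentHp to health divided by 100, printing the result or "No" if the cast fails.
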(event Game|Damage|EventAnyDamage
  (params (Damage :type Float%20%28single-precision%29) (DamageType :type Damage%20Type%20Object%20Reference) (InstigatedBy :type Controller%20Object%20Reference) (DamageCauser :type Actor%20Object%20Reference))
  (bind _output_get (Variables|Default|SetCurrentHp (- (Variables|Default|GetCurrentHp) Damage)))
  (Rendering|Components|TextRender|SetText (Variables|Default|GetTextRender) (Utilities|Text|ToText(Float) _output_get "HalfToEven"))
  (bind _asdummy_widget (Utilities|Casting|CastToDummyWidget (UserInterface|GetWidget (Variables|Default|GetWidget)))
    (:then
      (bind _output_get_2 (Variables|/Game/HelloUnreal/Blueprints/DummyWidget.DummyWidget_C|SetCurrentHp _asdummy_widget (/ (Variables|Default|GetCurrentHp) 1e+02)))
      (Development|PrintString (Utilities|String|ToString(Float) _output_get_2)))
    (:CastFailed
      (Development|PrintString "No"))))

(fn ConstructionScript)