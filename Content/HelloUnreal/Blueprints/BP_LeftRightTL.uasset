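; BP_LeftRightTL is an actor Blueprint that slides its Cube back and forth using a Timeline.
; On BeginPlay it plays or reverses the Timeline depending on IsMoveRight.
; Each update sets the Cube's relative location to the Timeline value times the Scene component's relative location, so that component marks the travel target.
; When the Timeline finishes, it flips IsMoveRight and repeats, creating a ping-pong loop without Event Tick.
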(event EventBeginPlay
  (if (Variables|Default|GetIsMoveRight) :!label _label
    ;[0.15 0.15 0.15 0.5] Timeline은 자체 Tick 내장
    (bind _value (Timeline|Timeline Play)
      (:Update
        (Transformation|SetRelativeLocation (Variables|Default|GetCube) (* _value (Variables|/Script/Engine.SceneComponent|GetRelativeLocation (Variables|Default|GetScene))) false false))
      (:Finished
        (Variables|Default|SetIsMoveRight (not (Variables|Default|GetIsMoveRight)))
        (goto _label)))
    (else
      (Timeline|Timeline Reverse))))

(fn ConstructionScript)