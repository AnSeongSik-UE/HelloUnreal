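; BP_Rect01 is a practice actor that moves its AAA component around a square path in the X/Z plane.
; While IsPlay is set, Tick switches on the MoveType enum, calls the matching move function and advances to the next direction at each bound.
; Each move function steps a stored coordinate by a fixed per-frame amount, without delta-time scaling, and applies it as relative location.
; EventPlay takes the play flag as input.
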(event EventTick
  (params (DeltaSeconds :type Float%20%28single-precision%29))
  ;[0.15 0.15 0.15 0.5] Tick
  (if (Variables|Default|GetbIsPlay)
    ;[0.15 0.15 0.15 0.5] N Cases, Enum
    (switch Utilities|FlowControl|Switch|SwitchonEN_MoveType (Variables|Default|GetMoveType)
      (:NewEnumerator2
        (CallFunction|MoveRight)
        ;[0.15 0.15 0.15 0.5] Switch
        (if (>= (Variables|Default|GetLocationX) 5e+02)
          (Variables|Default|SetMoveType "NewEnumerator4")))
      (:NewEnumerator4
        (CallFunction|MoveUp)
        (if (>= (Variables|Default|GetLocationZ) 5e+02)
          (Variables|Default|SetMoveType "NewEnumerator3")))
      (:NewEnumerator3
        (CallFunction|MoveLeft)
        (if (<= (Variables|Default|GetLocationX) 0.0)
          (Variables|Default|SetMoveType "NewEnumerator0")))
      (:NewEnumerator0
        (CallFunction|MoveDown)
        (if (<= (Variables|Default|GetLocationZ) 0.0)
          (Variables|Default|SetMoveType "NewEnumerator2"))))))

(event EventBeginPlay
  ;[0.15 0.15 0.15 0.5] 이 액터가 플레이 될 때
  ;[0.15 0.15 0.15 0.5] 화면에 String 출력
  (Development|PrintString "Hello"))

(fn ConstructionScript)

(fn MoveRight
  ;[0.15 0.15 0.15 0.5] Move X to +, Right
  (bind _output_get (Variables|Default|SetLocationX (+ (Variables|Default|GetLocationX) 1.0)))
  (Transformation|SetRelativeLocation (Variables|Default|GetAAA) (Math|Vector|MakeVector _output_get 0.0 (Variables|Default|GetLocationZ)) false false))

(fn MoveUp
  ;[0.15 0.15 0.15 0.5] Move Z to +, Up
  (bind _output_get (Variables|Default|SetLocationZ (+ (Variables|Default|GetLocationZ) 1.0)))
  (Transformation|SetRelativeLocation (Variables|Default|GetAAA) (Math|Vector|MakeVector (Variables|Default|GetLocationX) 0.0 _output_get) false false))

(fn MoveLeft
  ;[0.15 0.15 0.15 0.5] Move X to -, Left
  (bind _output_get (Variables|Default|SetLocationX (+ (Variables|Default|GetLocationX) -1.0)))
  (Transformation|SetRelativeLocation (Variables|Default|GetAAA) (Math|Vector|MakeVector _output_get 0.0 (Variables|Default|GetLocationZ)) false false))

(fn MoveDown
  ;[0.15 0.15 0.15 0.5] Move Z to -, Down
  (bind _output_get (Variables|Default|SetLocationZ (+ (Variables|Default|GetLocationZ) -1.0)))
  (Transformation|SetRelativeLocation (Variables|Default|GetAAA) (Math|Vector|MakeVector (Variables|Default|GetLocationX) 0.0 _output_get) false false))

(fn EventPlay
  (params (bIsPlay :type Boolean))
  (Variables|Default|SetbIsPlay bIsPlay)
  (return false))