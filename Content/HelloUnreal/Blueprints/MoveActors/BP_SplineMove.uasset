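; BP_SplineMove is an actor Blueprint that moves a Cube along its Spline in a repeating loop.
; A Timeline value scales the spline length into a distance, and the world location at that distance positions the cube without following the spline's rotation.
; The Timeline restarts from the beginning when it finishes.
; EventPlay takes a boolean to start or resume the motion through DoPlay, or halt it through DoStop.
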(event Custom|DoStop
  (bind _value (Timeline|Timeline Stop)
    (:Update
      (Transformation|SetWorldLocationAndRotation (Variables|Default|GetCube) (.location (Spline|GetTransformatDistanceAlongSpline (Variables|Default|GetSpline) (* (Spline|GetSplineLength (Variables|Default|GetSpline)) _value) "World" false)) "0, 0, 0" false false))
    (:Finished
      (Timeline|Timeline PlayFromStart))))

(event Custom|DoPlay
  (bind _value (Timeline|Timeline Play)
    (:Update
      (Transformation|SetWorldLocationAndRotation (Variables|Default|GetCube) (.location (Spline|GetTransformatDistanceAlongSpline (Variables|Default|GetSpline) (* (Spline|GetSplineLength (Variables|Default|GetSpline)) _value) "World" false)) "0, 0, 0" false false))
    (:Finished
      (Timeline|Timeline PlayFromStart))))

(fn ConstructionScript)

(fn EventPlay
  (params (bIsPlay :type Boolean))
  (if bIsPlay
    (CallFunction|DoPlay)
    (else
      (CallFunction|DoStop)))
  (return false))