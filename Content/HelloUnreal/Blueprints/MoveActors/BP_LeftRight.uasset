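; Actor that slides its AAA component back and forth along the relative X axis between fixed limits while playing.
; Tick calls MoveRight or MoveLeft based on IsMoveRight, flipping it at each limit; the step is fixed per frame, not scaled by delta time.
; EventPlay and EventStop toggle the movement through IsPlay.
; The construction script gives AAA a dynamic material instance with a configurable Color; BeginPlay only prints a string.
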(event EventTick
  (params (DeltaSeconds :type Float%20%28single-precision%29))
  (if (Variables|Default|GetbIsPlay)
    (if (Variables|Default|GetbIsMoveRight)
      (CallFunction|MoveRight)
      (if (>= (Variables|Default|GetLocationX) 5e+02)
        (Variables|Default|SetbIsMoveRight false))
      (else
        (CallFunction|MoveLeft)
        (if (<= (Variables|Default|GetLocationX) 0.0)
          (Variables|Default|SetbIsMoveRight true))))))

(event EventEventPlay
  (Variables|Default|SetbIsPlay true))

(event EventEventStop
  (Variables|Default|SetbIsPlay false))

(event EventBeginPlay
  ;[0.15 0.15 0.15 0.5] 이 액터가 플레이 될 때
  ;[0.15 0.15 0.15 0.5] 화면에 String 출력
  (Development|PrintString "Hello"))

(fn ConstructionScript
  (bind _returnvalue (Rendering|Material|CreateDynamicMaterialInstance (Variables|Default|GetAAA) 0 "/Game/HelloUnreal/StartUnreal/M_Mask_Inst1.M_Mask_Inst1" "None" :!class /Script/Engine.PrimitiveComponent))
  (Rendering|Material|SetVectorParameterValue _returnvalue "Color" (Variables|Default|GetValue) :!class /Script/Engine.MaterialInstanceDynamic))

(fn MoveRight
  ;[0.15 0.15 0.15 0.5] Move X to +, Right
  (bind _output_get (Variables|Default|SetLocationX (+ (Variables|Default|GetLocationX) 1.0)))
  (Transformation|SetRelativeLocation (Variables|Default|GetAAA) (Math|Vector|MakeVector _output_get 0.0 0.0) false false))

(fn MoveLeft
  ;[0.15 0.15 0.15 0.5] Move X to -, Left
  (bind _output_get (Variables|Default|SetLocationX (+ (Variables|Default|GetLocationX) -1.0)))
  (Transformation|SetRelativeLocation (Variables|Default|GetAAA) (Math|Vector|MakeVector _output_get 0.0 0.0) false false))