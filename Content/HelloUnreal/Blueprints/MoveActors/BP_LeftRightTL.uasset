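; BP_LeftRightTL is an actor that slides a Cube back and forth with a Timeline, started and stopped by a linked Switch.
; BeginPlay binds to the Switch's play/stop dispatcher, or prints a red warning if none is connected.
; The Timeline scales the Scene component's relative location to position the Cube, flipping direction on each finish.
; EventPlayStop and EventPlay both route a boolean to DoPlay or DoStop.
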(event Custom|DoPlay
  (if (Variables|Default|GetbIsMoveRight) :!label _label
    ;[0.15 0.15 0.15 0.5] Timeline은 자체 Tick 내장
    (bind _value (Timeline|Timeline Play)
      (:Update
        (Transformation|SetRelativeLocation (Variables|Default|GetCube) (* _value (Variables|/Script/Engine.SceneComponent|GetRelativeLocation (Variables|Default|GetScene))) false false))
      (:Finished
        (Variables|Default|SetbIsMoveRight (not (Variables|Default|GetbIsMoveRight)))
        (goto _label)))
    (else
      (Timeline|Timeline Reverse))))

(event Custom|DoStop
  ;[0.15 0.15 0.15 0.5] Timeline은 자체 Tick 내장
  (bind _value (Timeline|Timeline Stop)
    (:Update
      (Transformation|SetRelativeLocation (Variables|Default|GetCube) (* _value (Variables|/Script/Engine.SceneComponent|GetRelativeLocation (Variables|Default|GetScene))) false false))
    (:Finished
      (Variables|Default|SetbIsMoveRight (not (Variables|Default|GetbIsMoveRight)))
      (if (Variables|Default|GetbIsMoveRight)
        (Timeline|Timeline Play)
        (else
          (Timeline|Timeline Reverse))))))

(event EventBeginPlay
  ;[0.15 0.15 0.15 0.5] EventDispatcher Bind
  (bind _switch (Variables|Default|GetSwitch)
    (:then
      (EventDispatchers|BindEventtoEventDispatcherPlayStop _switch (EventDispatchers|CreateEvent :!event EventPlayStop)))
    (:else
      (Development|PrintString (Utilities|String|Append (Utilities|GetDisplayName self) " not connected at Switch") true true "(R=1.000000,G=0.000000,B=0.000000,A=1.000000)"))))

(fn ConstructionScript)

(fn EventPlayStop
  (params (bToggle :type Boolean))
  (if bToggle
    (CallFunction|DoPlay)
    (else
      (CallFunction|DoStop))))

(fn EventPlay
  (params (bIsPlay :type Boolean))
  (if bIsPlay
    (CallFunction|DoPlay)
    (else
      (CallFunction|DoStop)))
  (return false))