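; BP_Rect02 is an actor that loops its AAA component along an L-shaped path in the X-Z plane.
; Tick switches on MoveType, stepping X or Z by a fixed amount and applying it as relative location, so speed depends on frame rate.
; Limit checks chain Right, Up, Down and Left, so the component retraces both legs instead of tracing a full rectangle.
; BeginPlay only prints a string.
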(event EventTick
  (params (DeltaSeconds :type Float%20%28single-precision%29))
  (switch Utilities|FlowControl|Switch|SwitchonEN_MoveType (Variables|Default|GetMoveType)
    (:NewEnumerator2
      ;[0.15 0.15 0.15 0.5] Move X to +, Right
      (bind _output_get (Variables|Default|SetLocationX (+ (Variables|Default|GetLocationX) 5.0)))
      (Transformation|SetRelativeLocation (Variables|Default|GetAAA) (Math|Vector|MakeVector _output_get 0.0 (Variables|Default|GetLocationZ)) false false)
      (if (>= (Variables|Default|GetLocationX) 5e+02)
        (Variables|Default|SetMoveType "NewEnumerator4")))
    (:NewEnumerator4
      ;[0.15 0.15 0.15 0.5] Move Z to +, Up
      (bind _output_get_2 (Variables|Default|SetLocationZ (+ (Variables|Default|GetLocationZ) 5.0)))
      (Transformation|SetRelativeLocation (Variables|Default|GetAAA) (Math|Vector|MakeVector (Variables|Default|GetLocationX) 0.0 _output_get_2) false false)
      (if (>= (Variables|Default|GetLocationZ) 5e+02)
        (Variables|Default|SetMoveType "NewEnumerator0")))
    (:NewEnumerator3
      ;[0.15 0.15 0.15 0.5] Move X to -, Left
      (bind _output_get_3 (Variables|Default|SetLocationX (+ (Variables|Default|GetLocationX) -5.0)))
      (Transformation|SetRelativeLocation (Variables|Default|GetAAA) (Math|Vector|MakeVector _output_get_3 0.0 (Variables|Default|GetLocationZ)) false false)
      (if (<= (Variables|Default|GetLocationX) 0.0)
        (Variables|Default|SetMoveType "NewEnumerator2")))
    (:NewEnumerator0
      ;[0.15 0.15 0.15 0.5] Move Z to -, Down
      (bind _output_get_4 (Variables|Default|SetLocationZ (+ (Variables|Default|GetLocationZ) -5.0)))
      (Transformation|SetRelativeLocation (Variables|Default|GetAAA) (Math|Vector|MakeVector (Variables|Default|GetLocationX) 0.0 _output_get_4) false false)
      (if (<= (Variables|Default|GetLocationZ) 0.0)
        (Variables|Default|SetMoveType "NewEnumerator3")))))

(event EventBeginPlay
  ;[0.15 0.15 0.15 0.5] 이 액터가 플레이 될 때
  ;[0.15 0.15 0.15 0.5] 화면에 String 출력
  (Development|PrintString "Hello"))

(fn ConstructionScript)