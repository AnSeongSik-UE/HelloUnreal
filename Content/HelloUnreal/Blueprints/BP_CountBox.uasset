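; BP_CountBox is a counter box that displays a number on a TextRender component.
; Each call to the ToggleCountBox event increments Count, or resets it to zero when IsLimited is set, then updates the text.
; IsLimited is re-evaluated after each update, so once the count reaches nine the following call wraps it back to zero.
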(event Custom|ToggleCountBox
  (if (Variables|Default|GetbIsLimited)
    ;[0.15 0.15 0.15 0.5] Set Counts
    (Variables|Default|SetCount 0)
    (else
      (bind _result (Math|Integer|IncrementInt (Variables|Default|GetCount))
        (:%20%20
          (bind _output_get (Variables|Default|SetCount _result))))))
  ;[0.15 0.15 0.15 0.5] Set Text
  (Rendering|Components|TextRender|SetText (Variables|Default|GetTextRender) (Utilities|Text|ToText(Integer) _output_get))
  ;[0.15 0.15 0.15 0.5] Condition Judgement
  (if (>= (Variables|Default|GetCount) 9)
    (Variables|Default|SetbIsLimited true)
    (else
      (Variables|Default|SetbIsLimited false))))

(fn ConstructionScript)